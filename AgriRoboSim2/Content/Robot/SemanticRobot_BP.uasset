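; Semantic stand-in for the robot arm that mirrors RobotBP's arm for segmentation image generation.
; It copies the arm's skeletal mesh onto a poseable mesh at BeginPlay and again on first tick, applying an unlit material, scene-capture-only visibility and the SegmentImageGen tag.
; Each tick it matches the arm's world transform and copies every bone transform in component space.
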(event EventBeginPlay
  (CallFunction|UpdateRobotArmMesh))

(event Collision|EventActorBeginOverlap
  (params (OtherActor :type Actor%20Object%20Reference)))

(event EventTick
  (params (DeltaSeconds :type Float%20%28single-precision%29))
  (CallFunction|UpdateJoints)
  (Utilities|FlowControl|DoOnce false
    (:Completed
      (CallFunction|UpdateRobotArmMesh))))

(fn ConstructionScript)

(fn UpdateRobotArmMesh
  (bind _poseablemesh (Variables|Default|GetPoseableMesh))
  (bind _poseablemesh_2 (Variables|Default|GetPoseableMesh))
  (Components|SkinnedMesh|SetSkinnedAssetandUpdate _poseablemesh_2 (Class|SkinnedMeshComponent|GetSkinnedAsset (Variables|/Game/Robot/Robot_BP.Robot_BP_C|GetArm (Variables|Default|GetRobotBP))) true)
  (for _index (range 0 (Rendering|Material|GetNumMaterials _poseablemesh_2))
    (Rendering|Material|SetMaterial _poseablemesh_2 _index "/Game/Assets/Materials/UnLitRobot_M.UnLitRobot_M")
    (Class|PrimitiveComponent|SetVisibleinSceneCaptureOnly _poseablemesh true)
    (Transformation|SetWorldTransform _poseablemesh (Transformation|GetWorldTransform (Variables|/Game/Robot/Robot_BP.Robot_BP_C|GetArm (Variables|Default|GetRobotBP))) false true)
    (Variables|Default|SetTags (Utilities|Array|MakeArray "SegmentImageGen"))))

(fn UpdateJoints
  (bind _robotbp (Variables|Default|GetRobotBP))
  (bind _robotbp_2 (Variables|Default|GetRobotBP))
  (bind _arm (Variables|/Game/Robot/Robot_BP.Robot_BP_C|GetArm _robotbp))
  (bind _arm_2 (Variables|/Game/Robot/Robot_BP.Robot_BP_C|GetArm _robotbp_2))
  (Transformation|SetWorldTransform (Variables|Default|GetPoseableMesh) (Transformation|GetWorldTransform _arm) false true)
  (if (Class|GameplayStatics|ObjectIsA (Class|SkinnedMeshComponent|GetSkinnedAsset (Variables|Default|GetPoseableMesh)) (Utilities|GetClass (Class|SkinnedMeshComponent|GetSkinnedAsset _arm)))
    (for _index (range 0 (Class|SkinnedMeshComponent|GetNumBones _arm_2))
      (Components|PoseableMesh|SetBoneTransformbyName (Variables|Default|GetPoseableMesh) (Class|SkinnedMeshComponent|GetBoneName _arm_2 _index) (Transformation|GetBoneTransform _arm_2 (Class|SkinnedMeshComponent|GetBoneName _arm_2 _index) "RTS_Component") "ComponentSpace"))))