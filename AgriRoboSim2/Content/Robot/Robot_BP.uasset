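; Robot actor that bridges a data-table-selected robot arm and its camera rig to ROS.
; On BeginPlay it swaps in the selected mesh and physics asset, attaches the CineCamera to the end-effector socket and initializes arm and camera ROS components.
; A looping timer captures two color and two depth scene captures and publishes them.
; Tick applies joint targets and tags the game state; GetRobotInfo returns a configuration and pose string.
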(event Custom|PubImage
  (Class|ROSCameraControl|UpdateAllCameraParameters (Variables|Default|GetROSCameraControl) (Variables|Default|GetCineCamera))
  (Rendering|SceneCapture|CaptureScene (Variables|Default|GetDepth) :!class /Script/Engine.SceneCaptureComponent2D)
  (Class|ROSCameraControl|PublishAllTopic (Variables|Default|GetROSCameraControl)))

(event EventBeginPlay
  (bind _arm (Variables|Default|GetArm))
  ;[0.3846 0.6517 1] Robot Swapping
  (bind _returnvalue (Utilities|GetDataTableRow (Variables|Default|GetRobotSelectionDataTable) (Variables|Default|GetRobotSelection))
    (:then
      (Variables|/Script/AgriRoboSim.ROSArmControl|SetJointTopicOrder (Variables|Default|GetROSArmControl) (Variables|Default|GetJoint%20Topic%20Order))
      (Components|SkeletalMesh|SetSkeletalMeshAsset _arm (.Robot (Utilities|Struct|BreakRobotSwap_S _returnvalue)))
      (Components|SkinnedMesh|SetPhysicsAsset _arm (.PhysicsAsset (Utilities|Struct|BreakRobotSwap_S _returnvalue)) true)
      (Transformation|AttachComponentToComponent (Variables|Default|GetCineCamera) (Variables|Default|GetArm) (.EEFSocketName (Utilities|Struct|BreakRobotSwap_S _returnvalue)) "KeepRelative" "KeepRelative" "KeepRelative" true)
      (Class|SceneComponent|AddWorldTransform (Variables|Default|GetArm) (.Transform (Utilities|Struct|BreakRobotSwap_S _returnvalue)) false true)
      (Class|ROSArmControl|InitRobotArm (Variables|Default|GetROSArmControl) (Variables|Default|GetArm) (.JointProfile (Utilities|Struct|BreakRobotSwap_S _returnvalue)) (.JointBoneName (Utilities|Struct|BreakRobotSwap_S _returnvalue)))
      (Variables|/Script/AgriRoboSim.ROS2NodeComponent|SetTopicPrefix (Variables|Default|GetROSCameraControl) (Variables|Default|GetTopic%20Prefix))
      (Rendering|SceneCapture|CaptureScene (Variables|Default|GetDepth) :!class /Script/Engine.SceneCaptureComponent2D)
      (Class|ROSCameraControl|InitROSTopics (Variables|Default|GetROSCameraControl) (Utilities|Map|MakeMap (Variables|Default|GetColor) (Utilities|Enum|LiteralenumECaptureType "ColorCapture") (Variables|Default|GetDepth) (Utilities|Enum|LiteralenumECaptureType "DepthCapture") (Variables|Default|GetColorOne) (Utilities|Enum|LiteralenumECaptureType "ColorCapture") (Variables|Default|GetDepthOne) (Utilities|Enum|LiteralenumECaptureType "DepthCapture")) (Variables|Default|GetCineCamera) (Variables|Default|GetImageWidth) (Variables|Default|GetImageHeight))
      (Utilities|Time|SetTimerbyEvent (delegate Custom|PubImage) (Variables|Default|GetImageMessagePeriod) true true 1.0))
    (:RowNotFound
      (Development|PrintString "Invalid Robot Selection Name" true true "(R=0.000000,G=0.660000,B=1.000000,A=1.000000)" 5.0))))

(event EventTick
  (params (DeltaSeconds :type Float%20%28single-precision%29))
  (Class|ROSArmControl|SetJointsTargets (Variables|Default|GetROSArmControl))
  (bind _asmain_game_state_base (Utilities|Casting|CastToMainGameStateBase (Game|GetGameState)))
  (GameplayTags|AddGameplayTag (Variables|/Game/Levels/GameModes/MainMenu/MainGameStateBase.MainGameStateBase_C|GetROSSceneInfoGameplayTags _asmain_game_state_base) "(TagName=\"ROSSceneInfo.RobotUpdate\")" :!class /Script/GameplayTags.BlueprintGameplayTagLibrary))

(fn ConstructionScript)

(fn GetRobotInfo
  (bind _color (Variables|Default|GetColor))
  (bind _returnvalue (Transformation|GetWorldTransform _color))
  (bind _rotation (Math|Transform|BreakTransform _returnvalue))
  (bind _returnvalue_2 (Math|Conversions|ToQuaternion(Rotator) _rotation))
  (bind _output_get (Variables|Default|SetInformation (Utilities|String|Append (Variables|Default|GetTopic%20Prefix) "," (Utilities|String|ToString(Name) (Variables|Default|GetRobotSelection)) "," (Utilities|String|ToString(Object) (Class|SkinnedMeshComponent|GetSkinnedAsset (Variables|Default|GetArm))) "," (Utilities|String|ToString(Transform) (Transformation|GetWorldTransform (Variables|Default|GetArm))) "," (Utilities|String|ToString(Float) (Variables|/Script/Engine.SceneCaptureComponent2D|GetFOVAngle (Variables|Default|GetColor))) "," (Utilities|String|ToString(Integer) (Variables|Default|GetImageHeight)) "," (Utilities|String|ToString(Integer) (Variables|Default|GetImageWidth)) "," (Utilities|String|ToString(Transform) _returnvalue) "," (Class|KismetStringLibrary|BuildStringDouble (Class|KismetStringLibrary|BuildStringDouble (Class|KismetStringLibrary|BuildStringDouble (Class|KismetStringLibrary|BuildStringDouble "Camera Quat: " "X=" (.x _returnvalue_2)) "Y=" (.y _returnvalue_2)) "Z=" (.z _returnvalue_2)) "W=" (.w _returnvalue_2)))))
  (return _output_get))