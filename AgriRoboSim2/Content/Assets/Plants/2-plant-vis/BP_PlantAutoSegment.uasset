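; Plant actor for paired color and segmentation image generation that spawns a second copy of itself as a segmentation twin on BeginPlay.
; SetPlant async-loads a mesh and segmentation texture, applies the mesh to the color actor and forwards the data to the twin.
; The twin swaps in dynamic materials carrying the segmentation texture and instance ID.
; Data table helpers look up plant meshes, scales, names and textures, wrapping variant indices.
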(event Custom|SetPlant
  (params (MeshSoftRef :type Static%20Mesh%20Soft%20Object%20Reference) (SegTexSoftRef :type Texture%20Soft%20Object%20Reference) (Name :type Text) (InstanceID :type Float%20%28double-precision%29) (Scale :type Float%20%28double-precision%29))
  (Utilities|AsyncLoadAsset MeshSoftRef
    (:Completed
      (Utilities|AsyncLoadAsset SegTexSoftRef
        (:Completed
          (Utilities|MaChangePlantbyDetail MeshSoftRef Scale Name SegTexSoftRef InstanceID))))))

(event Custom|SetSegmentation
  (params (Input :type Static%20Mesh%20Soft%20Object%20Reference) (A :type Float%20%28double-precision%29) (Input2 :type Texture%20Soft%20Object%20Reference) (InputPin :type Float%20%28double-precision%29))
  (Utilities|MaUpdateSegmentation Input A Input2 InputPin))

(event EventBeginPlay
  (if (Variables|Default|GetIsSegment)
    (Variables|Default|SetTags (Utilities|Array|MakeArray "SegmentImageGen"))
    (Variables|Default|SetSegmentationRef 0)
    (else
      (bind _returnvalue (Game|SpawnActorfromClass "BP_PlantAutoSegment_C" (Transformation|GetWorldTransform (Variables|Default|GetPlantMesh)) "Undefined" "MultiplyWithRoot" self true (Variables|Default|GetCurrentInstanceID) 0))
      (Variables|Default|SetTags (Utilities|Array|MakeArray "ColoredImageGen"))
      (Variables|Default|SetSegmentationRef _returnvalue))))

(fn ConstructionScript)

(fn ChangePlant
  (params (PlantSelection :type Integer) (ClearOpactiy :type Boolean))
  (bind _plantmesh (Variables|Default|GetPlantMesh))
  (bind _returnvalue (Utilities|GetDataTableRow "/Game/Assets/Plants/2-plant-vis/PlantArrCollection_DT.PlantArrCollection_DT" (Utilities|String|StringToName (Utilities|String|ToString(Integer) PlantSelection)))
    (:then
      (bind _keys (Utilities|Map|Keys (.MeshScaleCollection (Utilities|Struct|BreakPlantAutoArr_S _returnvalue))))
      (bind _values (Utilities|Map|Values (.MeshScaleCollection (Utilities|Struct|BreakPlantAutoArr_S _returnvalue))))
      (bind _keys_2 (Utilities|Map|Keys (.SegmentationTextCollection (Utilities|Struct|BreakPlantAutoArr_S _returnvalue))))
      (bind _values_2 (Utilities|Map|Values (.SegmentationTextCollection (Utilities|Struct|BreakPlantAutoArr_S _returnvalue))))
      (Components|StaticMesh|SetStaticMesh (Variables|Default|GetMeshHold) (Utilities|ResolveSoftReference (Utilities|Array|Get(acopy) _keys)))
      (Components|StaticMesh|SetStaticMesh _plantmesh (Utilities|ResolveSoftReference (Utilities|Array|Get(acopy) _keys)))
      (Transformation|SetWorldScale3D _plantmesh (Math|Conversions|ToVector(Float) (Utilities|Array|Get(acopy) _values)))
      (Utilities|FlowControl|Sequence
        (:then_0
          (if (Actor|ActorHasTag "ColoredImageGen")
            (return (Utilities|String|ToString(Text) (Utilities|Array|Get(acopy) _values_2)))))
        (:then_1
          (if (Actor|ActorHasTag "SegmentImageGen")
            (Class|PrimitiveComponent|SetVisibleinSceneCaptureOnly (Variables|Default|GetPlantMesh) true)
            (for (_array_element _array_index) (Rendering|Material|GetMaterials (Variables|Default|GetMeshHold))
              (bind _returnvalue_2 (Rendering|Material|CreateDynamicMaterialInstance _array_element "Temp" "None" :!class /Script/Engine.KismetMaterialLibrary))
              (Rendering|Material|SetScalarParameterValue _returnvalue_2 "OpacityIntensity" 0.2 :!class /Script/Engine.MaterialInstanceDynamic)
              (Rendering|Material|SetTextureParameterValue _returnvalue_2 "Albedo" (Utilities|ResolveSoftReference (Utilities|Array|Get(acopy) _keys_2)))
              (Rendering|Material|SetMaterial (Variables|Default|GetPlantMesh) _array_index _returnvalue_2)
              (return (Utilities|String|ToString(Text) (Utilities|Array|Get(acopy) _values_2))))))))
    (:RowNotFound
      (return "PlantNotFound"))))

(fn ChangePlantbyDetail
  (params (Mesh :type Static%20Mesh%20Soft%20Object%20Reference) (Scale :type Float%20%28double-precision%29) (Name :type Text) (Segment :type Texture%20Soft%20Object%20Reference) (InstanceID :type Float%20%28double-precision%29))
  (bind _outputpin (Utilities|MaChangePlantbyDetail Mesh Scale Name Segment InstanceID)
    (:color
      (return _outputpin))
    (:segment
      (return _outputpin))))

(fn GrabPlantDetail
  (params (Plant :type Integer) (NameVariant :type Integer) (MeshVariant :type Integer))
  (bind _dt (LocalVariables|GetDT))
  (bind _outrownames (DataTable|GetDataTableRowNames _dt))
  (bind _returnvalue (Utilities|GetDataTableRow _dt (Utilities|String|StringToName (Utilities|String|ToString(Integer) (+ (Math|Integer|%(Integer) Plant (Utilities|Array|Length _outrownames)) 1))))
    (:then
      ;[1 1 1] NameVar
      (bind _keys (Utilities|Map|Keys (.SegmentationTextCollection (Utilities|Struct|BreakPlantAutoArr_S _returnvalue))))
      (bind _values (Utilities|Map|Values (.SegmentationTextCollection (Utilities|Struct|BreakPlantAutoArr_S _returnvalue))))
      ;[1 1 1] MeshVar
      (bind _keys_2 (Utilities|Map|Keys (.MeshScaleCollection (Utilities|Struct|BreakPlantAutoArr_S _returnvalue))))
      (bind _values_2 (Utilities|Map|Values (.MeshScaleCollection (Utilities|Struct|BreakPlantAutoArr_S _returnvalue))))
      (return (Utilities|Array|Get(acopy) _keys_2 (Math|Integer|%(Integer) MeshVariant (Utilities|Map|Length (.MeshScaleCollection (Utilities|Struct|BreakPlantAutoArr_S _returnvalue))))) (Utilities|Array|Get(acopy) _values_2 (Math|Integer|%(Integer) MeshVariant (Utilities|Map|Length (.MeshScaleCollection (Utilities|Struct|BreakPlantAutoArr_S _returnvalue))))) (Utilities|Array|Get(acopy) _values (Math|Integer|%(Integer) NameVariant (Utilities|Map|Length (.SegmentationTextCollection (Utilities|Struct|BreakPlantAutoArr_S _returnvalue))))) (Utilities|Array|Get(acopy) _keys (Math|Integer|%(Integer) NameVariant (Utilities|Map|Length (.SegmentationTextCollection (Utilities|Struct|BreakPlantAutoArr_S _returnvalue))))) (Math|Integer|%(Integer) NameVariant (Utilities|Map|Length (.SegmentationTextCollection (Utilities|Struct|BreakPlantAutoArr_S _returnvalue)))) (Math|Integer|%(Integer) MeshVariant (Utilities|Map|Length (.MeshScaleCollection (Utilities|Struct|BreakPlantAutoArr_S _returnvalue)))) (Variables|Default|GetIsSegment)))
    (:RowNotFound
      (Development|PrintString (Utilities|String|ToString(Integer) (+ (Math|Integer|%(Integer) Plant (Utilities|Array|Length _outrownames)) 1)))
      (Development|PrintString "Plant ROW Not Found" true true "(R=1.000000,G=0.000000,B=0.068469,A=1.000000)"))))

(fn GrabPlant
  (params (ID :type Integer))
  (Development|PrintString "Change Plant")
  (bind _returnvalue (Utilities|GetDataTableRow "/Game/Assets/Plants/2-plant-vis/PlantArrCollection_DT.PlantArrCollection_DT" (Utilities|String|StringToName (Utilities|String|ToString(Integer) ID)))
    (:then
      (bind _keys (Utilities|Map|Keys (.MeshScaleCollection (Utilities|Struct|BreakPlantAutoArr_S _returnvalue))))
      (bind _values (Utilities|Map|Values (.MeshScaleCollection (Utilities|Struct|BreakPlantAutoArr_S _returnvalue))))
      (bind _keys_2 (Utilities|Map|Keys (.SegmentationTextCollection (Utilities|Struct|BreakPlantAutoArr_S _returnvalue))))
      (bind _values_2 (Utilities|Map|Values (.SegmentationTextCollection (Utilities|Struct|BreakPlantAutoArr_S _returnvalue))))
      (return (Utilities|Array|Get(acopy) _keys ID) (Utilities|Array|Get(acopy) _keys_2 ID) (Utilities|Array|Get(acopy) _values_2 ID) (Utilities|Array|Get(acopy) _values ID)))
    (:RowNotFound
      (return 0 0 "" 0.0))))