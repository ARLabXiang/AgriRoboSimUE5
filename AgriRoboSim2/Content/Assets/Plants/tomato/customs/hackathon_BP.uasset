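; Tomato plant scene actor that procedurally generates its content through a PCG component at BeginPlay.
; GeneratePCG cleans up, applies a seed and generates, then waits a fixed delay before having the tomato disease game state register tomatoes and assign plant instance IDs.
; A separate SetFilteredDisease helper recursively trims trailing entries from a comma-separated disease string, with the recursive call using a hardcoded element limit.
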(event Custom|GeneratePCG
  (params (Seed :type Integer))
  (bind _pcg (Variables|Default|GetPCG))
  (Class|PCGComponent|Cleanup _pcg true false)
  (Variables|/Script/PCG.PCGComponent|SetSeed _pcg Seed)
  (PCG|Generate _pcg true)
  (Utilities|FlowControl|Delay 2.0)
  (bind _asmain_game_state_base_tomato_disease (Utilities|Casting|CastToMainGameStateBaseTomatoDisease (Game|GetGameState)))
  (Default|RegisterTomatosinScene _asmain_game_state_base_tomato_disease)
  (Default|AssignPlantInstanceID _asmain_game_state_base_tomato_disease))

(event EventBeginPlay
  (CallFunction|GeneratePCG 0))

(event Collision|EventActorBeginOverlap
  (params (OtherActor :type Actor%20Object%20Reference)))

(event EventTick
  (params (DeltaSeconds :type Float%20%28single-precision%29)))

(fn ConstructionScript)

(fn SetFilteredDisease
  (params (FilteredDisease :type String) (MaxElements :type Integer))
  (if (<= (Utilities|Array|Length (Utilities|String|ParseIntoArray FilteredDisease ",")) MaxElements)
    (Variables|Default|SetFilteredDisease FilteredDisease)
    (else
      (CallFunction|SetFilteredDisease (.LeftS (Utilities|String|Split FilteredDisease "," "IgnoreCase" "FromEnd")) 9))))